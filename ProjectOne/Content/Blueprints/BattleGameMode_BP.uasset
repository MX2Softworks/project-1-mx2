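; Battle game mode that keeps the seven-slot turn order widget in sync while the player controller is engaged.
; Tick draws the order once, then polls BattleManager's attack flag to play the widget animation, clear the flag and redraw.
; Redraws start from the last valid entry before the turn counter.
; Slots get Soul_Orb for MainCharacter or Sluagh art for Sluagh, with leftovers padded by Reticle.
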(event EventTick
  (params (DeltaSeconds :type Float%20%28single-precision%29))
  (bind _asbattle_player_controller_bp (Utilities|Casting|CastToBattlePlayerController_BP (Game|GetPlayerController 0)))
  (if (Variables|/Game/Blueprints/BattlePlayerController_BP.BattlePlayerController_BP_C|GetIsEngaged _asbattle_player_controller_bp)
    (if (Variables|Default|GetDrewInitial)
      (bind _returnvalue (Class|BattleManager|GetAttackOccurredBP (Variables|Default|GetBattleManager)))
      (if _returnvalue
        (bind _foundwidgets (Widget|GetAllWidgetsOfClass "/Game/Blueprints/Widgets/TurnOrderWidget_BP.TurnOrderWidget_BP_C" true))
        (bind _asturn_order_widget_bp (Utilities|Casting|CastToTurnOrderWidget_BP (Utilities|Array|Get(acopy) _foundwidgets)))
        (bind _output_get (Variables|Default|SetTurnOrderWidget _asturn_order_widget_bp))
        (Default|TurnOrderAnimations _output_get)
        (Development|PrintString "Animation")
        (Class|BattleManager|SetAttackOccurredBP (Variables|Default|GetBattleManager) false)
        (bind _returnvalue_2 (Class|BattleManager|GetTurnCounter (Variables|Default|GetBattleManager)))
        (bind _output_get_2 (Variables|Default|SetLastCharPosition (- _returnvalue_2 1)))
        (bind _returnvalue_3 (Class|BattleManager|GetTurnOrderWidgetArray (Variables|Default|GetBattleManager)))
        (while (not (Utilities|IsValid (Utilities|Array|Get(acopy) _returnvalue_3 _output_get_2)))
          (Variables|Default|SetLastCharPosition (- (Variables|Default|GetLastCharPosition) 1)))
        (Variables|Default|SetFirstIndex (Variables|Default|GetLastCharPosition))
        (Class|BattleManager|GetTurnCounter (Variables|Default|GetBattleManager) :!label _label)
        (bind _returnvalue_4 (Class|BattleManager|GetTurnOrderWidgetArray (Variables|Default|GetBattleManager)))
        (bind _output_get_3 (Variables|Default|SetTurnOrder _returnvalue_4))
        (for _index (range (Variables|Default|GetFirstIndex) (- (Utilities|Array|Length _output_get_3) 1))
          (Utilities|Casting|CastToMainCharacter (Utilities|Array|Get(acopy) (Variables|Default|GetTurnOrder) _index)
            (:then
              (bind _foundwidgets_2 (Widget|GetAllWidgetsOfClass "/Game/Blueprints/Widgets/TurnOrderWidget_BP.TurnOrderWidget_BP_C" true))
              (bind _asturn_order_widget_bp_2 (Utilities|Casting|CastToTurnOrderWidget_BP (Utilities|Array|Get(acopy) _foundwidgets_2)))
              (Variables|Default|SetTurnOrderWidget _asturn_order_widget_bp_2)
              (switch int (Variables|Default|GetOrderPortraitsDisplayed)
                (:0
                  (Variables|/Game/Blueprints/Widgets/TurnOrderWidget_BP.TurnOrderWidget_BP_C|SetOrderOne (Variables|Default|GetTurnOrderWidget) "/Game/Assets/Textures/Soul_Orb.Soul_Orb"))
                (:1
                  (Variables|/Game/Blueprints/Widgets/TurnOrderWidget_BP.TurnOrderWidget_BP_C|SetOrderTwo (Variables|Default|GetTurnOrderWidget) "/Game/Assets/Textures/Soul_Orb.Soul_Orb"))
                (:2
                  (Variables|/Game/Blueprints/Widgets/TurnOrderWidget_BP.TurnOrderWidget_BP_C|SetOrderThree (Variables|Default|GetTurnOrderWidget) "/Game/Assets/Textures/Soul_Orb.Soul_Orb"))
                (:3
                  (Variables|/Game/Blueprints/Widgets/TurnOrderWidget_BP.TurnOrderWidget_BP_C|SetOrderFour (Variables|Default|GetTurnOrderWidget) "/Game/Assets/Textures/Soul_Orb.Soul_Orb"))
                (:4
                  (Variables|/Game/Blueprints/Widgets/TurnOrderWidget_BP.TurnOrderWidget_BP_C|SetOrderFive (Variables|Default|GetTurnOrderWidget) "/Game/Assets/Textures/Soul_Orb.Soul_Orb"))
                (:5
                  (Variables|/Game/Blueprints/Widgets/TurnOrderWidget_BP.TurnOrderWidget_BP_C|SetOrderSix (Variables|Default|GetTurnOrderWidget) "/Game/Assets/Textures/Soul_Orb.Soul_Orb"))
                (:6
                  (Variables|/Game/Blueprints/Widgets/TurnOrderWidget_BP.TurnOrderWidget_BP_C|SetOrderSeven (Variables|Default|GetTurnOrderWidget) "/Game/Assets/Textures/Soul_Orb.Soul_Orb")))
              (Variables|Default|SetOrderPortraitsDisplayed (+ (Variables|Default|GetOrderPortraitsDisplayed) 1)))
            (:CastFailed
              (Utilities|Casting|CastToSluagh (Utilities|Array|Get(acopy) (Variables|Default|GetTurnOrder) _index))
              (bind _foundwidgets_3 (Widget|GetAllWidgetsOfClass "/Game/Blueprints/Widgets/TurnOrderWidget_BP.TurnOrderWidget_BP_C" true))
              (bind _asturn_order_widget_bp_3 (Utilities|Casting|CastToTurnOrderWidget_BP (Utilities|Array|Get(acopy) _foundwidgets_3)))
              (Variables|Default|SetTurnOrderWidget _asturn_order_widget_bp_3)
              (switch int (Variables|Default|GetOrderPortraitsDisplayed)
                (:0
                  (Variables|/Game/Blueprints/Widgets/TurnOrderWidget_BP.TurnOrderWidget_BP_C|SetOrderOne (Variables|Default|GetTurnOrderWidget) "/Game/Assets/Textures/Sluagh.Sluagh"))
                (:1
                  (Variables|/Game/Blueprints/Widgets/TurnOrderWidget_BP.TurnOrderWidget_BP_C|SetOrderTwo (Variables|Default|GetTurnOrderWidget) "/Game/Assets/Textures/Sluagh.Sluagh"))
                (:2
                  (Variables|/Game/Blueprints/Widgets/TurnOrderWidget_BP.TurnOrderWidget_BP_C|SetOrderThree (Variables|Default|GetTurnOrderWidget) "/Game/Assets/Textures/Sluagh.Sluagh"))
                (:3
                  (Variables|/Game/Blueprints/Widgets/TurnOrderWidget_BP.TurnOrderWidget_BP_C|SetOrderFour (Variables|Default|GetTurnOrderWidget) "/Game/Assets/Textures/Sluagh.Sluagh"))
                (:4
                  (Variables|/Game/Blueprints/Widgets/TurnOrderWidget_BP.TurnOrderWidget_BP_C|SetOrderFive (Variables|Default|GetTurnOrderWidget) "/Game/Assets/Textures/Sluagh.Sluagh"))
                (:5
                  (Variables|/Game/Blueprints/Widgets/TurnOrderWidget_BP.TurnOrderWidget_BP_C|SetOrderSix (Variables|Default|GetTurnOrderWidget) "/Game/Assets/Textures/Sluagh.Sluagh"))
                (:6
                  (Variables|/Game/Blueprints/Widgets/TurnOrderWidget_BP.TurnOrderWidget_BP_C|SetOrderSeven (Variables|Default|GetTurnOrderWidget) "/Game/Assets/Textures/Sluagh.Sluagh")))
              (Variables|Default|SetOrderPortraitsDisplayed (+ (Variables|Default|GetOrderPortraitsDisplayed) 1)))))
        (if (< (Variables|Default|GetOrderPortraitsDisplayed) 7)
          (for _index_2 (range (Variables|Default|GetOrderPortraitsDisplayed) 6)
            (bind _foundwidgets_4 (Widget|GetAllWidgetsOfClass "/Game/Blueprints/Widgets/TurnOrderWidget_BP.TurnOrderWidget_BP_C" true))
            (bind _asturn_order_widget_bp_4 (Utilities|Casting|CastToTurnOrderWidget_BP (Utilities|Array|Get(acopy) _foundwidgets_4)))
            (Variables|Default|SetTurnOrderWidget _asturn_order_widget_bp_4)
            (switch int (Variables|Default|GetOrderPortraitsDisplayed)
              (:0
                (Variables|/Game/Blueprints/Widgets/TurnOrderWidget_BP.TurnOrderWidget_BP_C|SetOrderOne (Variables|Default|GetTurnOrderWidget) "/Game/Assets/Textures/reticle.reticle"))
              (:1
                (Variables|/Game/Blueprints/Widgets/TurnOrderWidget_BP.TurnOrderWidget_BP_C|SetOrderTwo (Variables|Default|GetTurnOrderWidget) "/Game/Assets/Textures/reticle.reticle"))
              (:2
                (Variables|/Game/Blueprints/Widgets/TurnOrderWidget_BP.TurnOrderWidget_BP_C|SetOrderThree (Variables|Default|GetTurnOrderWidget) "/Game/Assets/Textures/reticle.reticle"))
              (:3
                (Variables|/Game/Blueprints/Widgets/TurnOrderWidget_BP.TurnOrderWidget_BP_C|SetOrderFour (Variables|Default|GetTurnOrderWidget) "/Game/Assets/Textures/reticle.reticle"))
              (:4
                (Variables|/Game/Blueprints/Widgets/TurnOrderWidget_BP.TurnOrderWidget_BP_C|SetOrderFive (Variables|Default|GetTurnOrderWidget) "/Game/Assets/Textures/reticle.reticle"))
              (:5
                (Variables|/Game/Blueprints/Widgets/TurnOrderWidget_BP.TurnOrderWidget_BP_C|SetOrderSix (Variables|Default|GetTurnOrderWidget) "/Game/Assets/Textures/reticle.reticle"))
              (:6
                (Variables|/Game/Blueprints/Widgets/TurnOrderWidget_BP.TurnOrderWidget_BP_C|SetOrderSeven (Variables|Default|GetTurnOrderWidget) "/Game/Assets/Textures/reticle.reticle")))
            (Variables|Default|SetOrderPortraitsDisplayed (+ (Variables|Default|GetOrderPortraitsDisplayed) 1)))
          (Variables|Default|SetOrderPortraitsDisplayed 0) ; Continue Tick Here
          (else
            (Variables|Default|SetOrderPortraitsDisplayed 0))))
      (elif (not (Variables|Default|GetDrewInitial))
        (bind _returnvalue_5 (Class|BattleManager|GetTurnCounter (Variables|Default|GetBattleManager)))
        (Variables|Default|SetFirstIndex _returnvalue_5)
        (Variables|Default|SetDrewInitial true)
        (goto _label)))))

(fn ConstructionScript)