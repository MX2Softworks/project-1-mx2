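; Player controller for battles that possesses the character named Beck and manages the turn-based battle UI.
; On BeginPlay it finds Beck by object name among GameCharacter actors and possesses it.
; While engaged, Tick polls the battle manager's turn and sets the game mode's attack or defense state.
; On the player's turn it shows the main battle widget with mouse input; otherwise it removes the main and attack widgets.
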(event EventBeginPlay
  (Variables|Default|SetIsUserInterfaceActive false) ; Sets is UI Active to False
  (CallFunction|FindBeck)
  (Pawn|Possess (Variables|Default|GetBeck)))

(event EventTick
  (params (DeltaSeconds :type Float%20%28single-precision%29))
  ;[1 1 1] Draws UI to Viewport
  (if (Variables|Default|GetIsEngaged)
    (bind _asbattle_game_mode_bp (Utilities|Casting|CastToBattleGameMode_BP (Game|GetGameMode)))
    (bind _output_get (Variables|Default|SetBattleGameMode _asbattle_game_mode_bp))
    (bind _returnvalue (Class|BattleManager|GetIsPlayerTurn (Variables|/Game/Blueprints/BattleGameMode_BP.BattleGameMode_BP_C|GetBattleManager _output_get)))
    (if _returnvalue
      (Variables|/Game/Blueprints/BattleGameMode_BP.BattleGameMode_BP_C|SetAttackState (Variables|Default|GetBattleGameMode) true)
      (Variables|/Game/Blueprints/BattleGameMode_BP.BattleGameMode_BP_C|SetDefenseState (Variables|Default|GetBattleGameMode) false)
      (if (not (Variables|Default|GetIsUserInterfaceActive))
        (Variables|Default|SetIsUserInterfaceActive true)
        (bind _returnvalue_2 (UserInterface|CreateWidget "/Game/Blueprints/Widgets/BattleMainWidget_BP.BattleMainWidget_BP_C"))
        (UserInterface|Viewport|AddtoViewport _returnvalue_2 0)
        (Variables|Default|SetbShowMouseCursor true)
        (bind _asbattle_player_controller_bp (Utilities|Casting|CastToBattlePlayerController_BP (Game|GetPlayerController 0)))
        (Input|SetInputModeGameandUI _asbattle_player_controller_bp _returnvalue_2 true false))
      (else
        (Variables|/Game/Blueprints/BattleGameMode_BP.BattleGameMode_BP_C|SetAttackState (Variables|Default|GetBattleGameMode) false)
        (Variables|/Game/Blueprints/BattleGameMode_BP.BattleGameMode_BP_C|SetDefenseState (Variables|Default|GetBattleGameMode) true)
        (bind _foundwidgets (Widget|GetAllWidgetsOfClass "/Game/Blueprints/Widgets/BattleMainWidget_BP.BattleMainWidget_BP_C" true))
        (Widget|RemovefromParent _foundwidgets)
        (bind _foundwidgets_2 (Widget|GetAllWidgetsOfClass "/Game/Blueprints/Widgets/BattleAttackWidget_BP.BattleAttackWidget_BP_C" true))
        (Widget|RemovefromParent _foundwidgets_2)
        (Variables|Default|SetIsUserInterfaceActive false)))))

(fn ConstructionScript)

(fn FindBeck
  (bind _outactors (Actor|GetAllActorsOfClass "/Script/ProjectOne.GameCharacter"))
  (for _array_element _outactors
    (if (Utilities|Name|Equal(Name) (Utilities|String|StringToName (Utilities|GetObjectName _array_element)) "Beck")
      (Variables|Default|SetBeck _array_element)
      (Development|PrintText "Beck Found!" true false)
      (return)))
  (return))