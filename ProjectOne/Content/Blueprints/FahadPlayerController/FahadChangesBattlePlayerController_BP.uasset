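; Battle test player controller that possesses the "Beck" character and opens the battle UI on demand.
; On BeginPlay it searches all GameCharacter actors for the object named "Beck", stores it and possesses it.
; The EngageTest input creates the main battle widget and shows the cursor, though its UI-active guard is never set true, so repeat presses add more widgets.
; Left mouse click only prints test text.
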(event EventBeginPlay
  (Variables|Default|SetbIsUserInterfaceActive false) ; Sets is UI Active to False
  (CallFunction|FindBeck)
  (Pawn|Possess (Variables|Default|GetBeck)))

(event EventTick
  (params (DeltaSeconds :type Float%20%28single-precision%29)))

(event Input|ActionEvents|InputActionEngageTest
  (params (Key :type Key%20Structure :default "AnyKey"))
  ;[1 1 1] Draws UI to Viewport upon pressing 'E'.
  (:Pressed
    ;;[1 1 1] Only draws UI if UI was not already drawn
    (if (not (Variables|Default|GetbIsUserInterfaceActive))
      (Variables|Default|SetbIsUserInterfaceActive false)
      (bind _returnvalue (UserInterface|CreateWidget "/Game/Blueprints/Widgets/BattleMainWidget_BP.BattleMainWidget_BP_C"))
      (UserInterface|Viewport|AddtoViewport _returnvalue 0)
      (Variables|Default|SetbShowMouseCursor true))))

(event Input|MouseEvents|LeftMouseButton
  (params (Key :type Key%20Structure :default "AnyKey"))
  ;[1 1 1] Testing mouse input. Feel free to remove.
  (:Pressed
    (Development|PrintText "Mouse Button Pressed")))

(fn ConstructionScript)

(fn FindBeck
  (bind _outactors (Actor|GetAllActorsOfClass "/Script/ProjectOne.GameCharacter"))
  (for _array_element _outactors
    (if (Utilities|Name|Equal(Name) (Utilities|String|StringToName (Utilities|GetObjectName _array_element)) "Beck")
      (Variables|Default|SetBeck _array_element)
      (Development|PrintText "Beck Found!" true false)
      (return)))
  (return))