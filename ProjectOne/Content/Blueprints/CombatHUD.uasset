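; CombatHUD is a HUD Blueprint that draws a reticle at the mouse cursor and reports whether the cursor targets a GameCharacter.
; DrawHUD centers a fixed-size reticle on the mouse position, offset by half the difference between HUD and viewport sizes.
; It also runs a complex Visibility trace under the cursor, using two flags to print hit or miss debug text only when the result changes.
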(event EventBeginPlay)

(event EventActorBeginOverlap
  (params (OtherActor :type Actor%20Object%20Reference)))

(event EventTick
  (params (DeltaSeconds :type Float%20%28single-precision%29)))

(event EventDrawHUD
  (params (SizeX :type Integer) (SizeY :type Integer))
  (bind _returnvalue (Game|GetPlayerController 0))
  (bind _returnvalue_2 (Math|Float|MakeLiteralFloat 32.0))
  (bind (_locationx _locationy) (Game|Player|GetMousePosition _returnvalue))
  (bind (_sizex _sizey) (HUD|GetViewportSize _returnvalue))
  (bind _returnvalue_3 (/ _returnvalue_2 2.0))
  (Canvas|DrawTexture "/Game/Sprites/Textures/reticle.reticle" (- (+ _locationx (/ (Math|Conversions|ToFloat(Integer) (- SizeX _sizex)) 2.0)) _returnvalue_3) (- (+ _locationy (/ (Math|Conversions|ToFloat(Integer) (- SizeY _sizey)) 2.0)) _returnvalue_3) _returnvalue_2 _returnvalue_2 0.0 0.0 1.0 1.0 "(R=1.000000,G=1.000000,B=1.000000,A=1.000000)")
  (Utilities|Casting|CastToGameCharacter (.HitActor (Collision|BreakHitResult (.HitResult (Game|Player|GetHitResultUnderCursorbyChannel _returnvalue "TraceTypeQuery1" true))))
    (:then
      (if (not (Variables|Default|GetGoodPrint))
        (Development|PrintText "Hitting Sluagh")
        (Variables|Default|SetBadPrint false)
        (Variables|Default|SetGoodPrint true)))
    (:CastFailed
      (if (not (Variables|Default|GetBadPrint))
        (Development|PrintText "Not Sluagh")
        (Variables|Default|SetGoodPrint false)
        (Variables|Default|SetBadPrint true)))))

(fn ConstructionScript)