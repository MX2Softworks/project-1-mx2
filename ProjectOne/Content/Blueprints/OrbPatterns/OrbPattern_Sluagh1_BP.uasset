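; Orb pattern actor for the Sluagh1 battle pattern, spawning a fixed number of soul orbs at timed intervals.
; BeginPlay shows a reticle at the mouse position, then after a delay plays a timeline whose sampled positions offset each orb spawned on Tick.
; Spawn origin comes from a downward camera trace, shifted using the vertical FOV.
; When the timeline finishes, it destroys the Terminator, fades out the reticle and removes itself.
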(event EventBeginPlay
  (Variables|Default|SetSpawn%20Timeline (Variables|Default|GetTimeline_0))
  (Variables|Default|SetPatternTime (Components|Timeline|GetTimelineLength (Variables|Default|GetSpawn%20Timeline)))
  (Variables|Default|SetIsFIrstTick true)
  (Variables|Default|SetTimer 0.4)
  (Variables|Default|SetTotalOrbs 11)
  (Variables|Default|SetCurrentOrbs 0)
  (if (not (Utilities|IsValid (Variables|Default|GetOrbReticle)))
    (bind _returnvalue (Game|SpawnActorfromClass "/Game/Blueprints/OrbReticle_BP.OrbReticle_BP_C" (Math|Transform|MakeTransform (+ (.WorldLocation (Game|Player|ConvertMouseLocationToWorldSpace (Game|GetPlayerController 0))) "0, 0,20.000000") "0, 0, 0" "0.250000,1.000000,0.250000") "Undefined" 0 0))
    (Variables|Default|SetOrbReticle _returnvalue)
    (Utilities|FlowControl|Delay 1.2)
    (Variables|Default|SetWaitForDelay_0 true)
    (bind _spawnpositions (Timeline|Timeline_0 Play)
      (:Finished
        (Actor|DestroyActor (Variables|Default|GetTerminator))
        (if (Utilities|IsValid (Variables|Default|GetOrbReticle))
          (Actor|DestroyActor (Variables|Default|GetOrbReticle))
          (Game|SpawnActorfromClass "/Game/Blueprints/OrbReticleFadeOut_BP.OrbReticleFadeOut_BP_C" (Math|Transform|MakeTransform (+ (.WorldLocation (Game|Player|ConvertMouseLocationToWorldSpace (Game|GetPlayerController 0))) "0, 0,20.000000") "0.000000,0.000000,90.000000" "0.250000,1.000000,0.250000") "Undefined" 0 0)
          (Utilities|FlowControl|Delay 1.5)
          (Actor|DestroyActor)
          (else
            (Actor|DestroyActor)))))))

(event EventTick
  (params (DeltaSeconds :type Float%20%28single-precision%29))
  (if (Variables|Default|GetIsFIrstTick)
    (bind _vertical_fov (CallFunction|GetVerticalFOV))
    (Variables|Default|SetVerticalFOV _vertical_fov)
    (bind _terminator (CallFunction|SpawnTerminator))
    (Variables|Default|SetTerminator _terminator)
    (bind _output_get (Variables|Default|SetIsFIrstTick false))
    (if (not _output_get)
      (bind _output_get_2 (Variables|Default|SetTimer (+ (Variables|Default|GetTimer) (Utilities|Time|GetWorldDeltaSeconds)) :!label _label))
      (if (and (>= (Variables|Default|GetTimer) 0.5) (< (Variables|Default|GetCurrentOrbs) (Variables|Default|GetTotalOrbs)))
        (if (Variables|Default|GetWaitForDelay_0)
          (Variables|Default|SetTimer 0.0)
          (CallFunction|SpawnOrb (stale EventBeginPlay _spawnpositions))
          (Variables|Default|SetCurrentOrbs (+ (Variables|Default|GetCurrentOrbs) 1)))))
    (else
      (goto _label))))

(fn ConstructionScript
  (|CallParentFunction))

(fn SpawnOrb
  (params (B :type Vector))
  (bind _asbattle_player_controller_bp (Utilities|Casting|CastToBattlePlayerController_BP (Game|GetPlayerController 0))
    (:then
      (bind _outhit (Collision|LineTraceByChannel (Transformation|GetActorLocation (Pawn|GetViewTarget _asbattle_player_controller_bp)) (Math|Vector|MakeVector (.X (Math|Vector|BreakVector (Transformation|GetActorLocation (Pawn|GetViewTarget _asbattle_player_controller_bp)))) (.Y (Math|Vector|BreakVector (Transformation|GetActorLocation (Pawn|GetViewTarget _asbattle_player_controller_bp)))) (- (.Z (Math|Vector|BreakVector (Transformation|GetActorLocation (Pawn|GetViewTarget _asbattle_player_controller_bp)))) 1e+04)) "TraceTypeQuery1" false 0 "None"))
      (bind _vertical_fov (CallFunction|GetVerticalFOV))
      (Game|SpawnActorfromClass "/Game/Blueprints/SoulOrbs/SoulOrb_BP.SoulOrb_BP_C" (Math|Transform|MakeTransform (+ (- (.Location (Collision|BreakHitResult _outhit)) (Math|Vector|MakeVector (* (Math|Vector|VectorLength (- (.TraceStart (Collision|BreakHitResult _outhit)) (.Location (Collision|BreakHitResult _outhit)))) (Math|Trig|Tan(Degrees) _vertical_fov)) 0.0 0.0)) B) "0.000000,0.000000,90.000000" "0.250000,1.000000,0.250000") "AlwaysSpawn" 0 0)
      (return))
    (:CastFailed
      (return))))