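; Orb pattern actor for battle that runs a timed wave of soul orbs, with a mouse-placed reticle and a screen-wide terminator bar.
; Tick spawns a capped number of orbs at a fixed interval, offset by the timeline's SpawnPositions.
; Downward traces from the view target and camera FOV math place orbs and terminator at opposite screen edges.
; When the timeline finishes, it destroys the terminator, reticle and itself.
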(event EventBeginPlay
  (Variables|Default|SetPatternTime (Components|Timeline|GetTimelineLength (Variables|Default|GetSpawn%20Timeline)))
  (Variables|Default|SetIsFIrstTick true)
  (Variables|Default|SetTimer 0.0)
  (Variables|Default|SetTotalOrbs 5)
  (Variables|Default|SetCurrentOrbs 0)
  (if (not (Utilities|IsValid (Variables|Default|GetOrbReticle)))
    (bind _returnvalue (Game|SpawnActorfromClass "/Game/Blueprints/OrbReticle_BP.OrbReticle_BP_C" (Math|Transform|MakeTransform (+ (.WorldLocation (Game|Player|ConvertMouseLocationToWorldSpace (Game|GetPlayerController 0))) "0, 0,20.000000") "0, 0, 0" "0.250000,1.000000,0.250000") "Undefined" 0 0))
    (Variables|Default|SetOrbReticle _returnvalue)
    (bind _spawnpositions (Timeline|Spawn%20Timeline Play)
      (:Finished
        (Utilities|FlowControl|Delay 0.01)
        (Actor|DestroyActor (Variables|Default|GetTerminator))
        (if (Utilities|IsValid (Variables|Default|GetOrbReticle))
          (Actor|DestroyActor (Variables|Default|GetOrbReticle))
          (Actor|DestroyActor)
          (else
            (Actor|DestroyActor)))))))

(event EventTick
  (params (DeltaSeconds :type Float%20%28single-precision%29))
  (if (Variables|Default|GetIsFIrstTick)
    (bind _vertical_fov (CallFunction|GetVerticalFOV))
    (Variables|Default|SetVerticalFOV _vertical_fov)
    (bind _terminator (SoulOrb|SpawnTerminator))
    (Variables|Default|SetTerminator _terminator)
    (bind _output_get (Variables|Default|SetIsFIrstTick false))
    (if (not _output_get)
      (bind _output_get_2 (Variables|Default|SetTimer (+ (Variables|Default|GetTimer) (Utilities|Time|GetWorldDeltaSeconds)) :!label _label))
      (if (and (>= (Variables|Default|GetTimer) 0.5) (< (Variables|Default|GetCurrentOrbs) (Variables|Default|GetTotalOrbs)))
        (Variables|Default|SetTimer 0.0)
        (SoulOrb|SpawnOrb (stale EventBeginPlay _spawnpositions))
        (Variables|Default|SetCurrentOrbs (+ (Variables|Default|GetCurrentOrbs) 1))))
    (else
      (goto _label))))

(fn ConstructionScript)

(fn GetVerticalFOV
  (bind _returnvalue (Game|GetPlayerController 0))
  (bind (_sizex _sizey) (HUD|GetViewportSize _returnvalue))
  ;[1 1 1] Calculates Vertical Field of View using the formula V = 2arctan(tan(H/2) * h/w)
  (return (Class|KismetMathLibrary|DegAtan (* (Math|Trig|Tan(Degrees) (/ (Camera|GetFOVAngle (Variables|/Script/Engine.PlayerController|GetPlayerCameraManager _returnvalue)) 2.0)) (/ (Math|Conversions|ToFloat(Integer) _sizey) (Math|Conversions|ToFloat(Integer) _sizex))))))

(fn SpawnOrb
  (params (B :type Vector))
  (bind _asbattle_player_controller_bp (Utilities|Casting|CastToBattlePlayerController_BP (Game|GetPlayerController 0))
    (:then
      (bind _outhit (Collision|LineTraceByChannel (Transformation|GetActorLocation (Pawn|GetViewTarget _asbattle_player_controller_bp)) (Math|Vector|MakeVector (.X (Math|Vector|BreakVector (Transformation|GetActorLocation (Pawn|GetViewTarget _asbattle_player_controller_bp)))) (.Y (Math|Vector|BreakVector (Transformation|GetActorLocation (Pawn|GetViewTarget _asbattle_player_controller_bp)))) (- (.Z (Math|Vector|BreakVector (Transformation|GetActorLocation (Pawn|GetViewTarget _asbattle_player_controller_bp)))) 1e+04)) "TraceTypeQuery1" false 0 "None"))
      (bind _vertical_fov (CallFunction|GetVerticalFOV))
      (Game|SpawnActorfromClass "/Game/Blueprints/SoulOrb_BP.SoulOrb_BP_C" (Math|Transform|MakeTransform (+ (- (.Location (Collision|BreakHitResult _outhit)) (Math|Vector|MakeVector (* (Math|Vector|VectorLength (- (.TraceStart (Collision|BreakHitResult _outhit)) (.Location (Collision|BreakHitResult _outhit)))) (Math|Trig|Tan(Degrees) _vertical_fov)) 0.0 0.0)) B) "0.000000,0.000000,90.000000" "0.250000,1.000000,0.250000") "AlwaysSpawn" 0 0)
      (return))
    (:CastFailed
      (return))))

(fn SpawnTerminator
  (bind _returnvalue (Game|GetPlayerController 0))
  ;[1 1 1] Draws a vertical line trace from the player's position down 10000 units until it hits the floor.
  (bind _asbattle_player_controller_bp (Utilities|Casting|CastToBattlePlayerController_BP _returnvalue)
    (:then
      (bind _outhit (Collision|LineTraceByChannel (Transformation|GetActorLocation (Pawn|GetViewTarget _asbattle_player_controller_bp)) (Math|Vector|MakeVector (.X (Math|Vector|BreakVector (Transformation|GetActorLocation (Pawn|GetViewTarget _asbattle_player_controller_bp)))) (.Y (Math|Vector|BreakVector (Transformation|GetActorLocation (Pawn|GetViewTarget _asbattle_player_controller_bp)))) (- (.Z (Math|Vector|BreakVector (Transformation|GetActorLocation (Pawn|GetViewTarget _asbattle_player_controller_bp)))) 1e+04)) "TraceTypeQuery1" false 0 "None"))
      ;[1 1 1] Uses the camera's vertical FOV to draw the terminator at the top of the screen. Uses the horizontal FOV to scale the bar so that it fits across the entire screen.
      (bind _returnvalue_2 (Game|SpawnActorfromClass "/Game/Blueprints/SoulTerminator_BP.SoulTerminator_BP_C" (Math|Transform|MakeTransform (+ (.Location (Collision|BreakHitResult _outhit)) (Math|Vector|MakeVector (* (Math|Trig|Tan(Degrees) (Variables|Default|GetVerticalFOV)) (Math|Vector|VectorLength (- (.TraceStart (Collision|BreakHitResult _outhit)) (.Location (Collision|BreakHitResult _outhit))))) 0.0 0.0)) "0.000000,90.000000,90.000000" (Math|Vector|MakeVector (* (* (Math|Vector|VectorLength (- (.TraceStart (Collision|BreakHitResult _outhit)) (.Location (Collision|BreakHitResult _outhit)))) (Math|Trig|Tan(Degrees) (/ (Camera|GetFOVAngle (Variables|/Script/Engine.PlayerController|GetPlayerCameraManager _returnvalue)) 2.0))) 2.0) 1.0 1.0)) "Undefined" 0 0))
      (return _returnvalue_2))
    (:CastFailed
      (return 0))))