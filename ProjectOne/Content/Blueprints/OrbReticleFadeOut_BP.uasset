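; Orb reticle fade-out sprite actor that tracks the mouse cursor while it fades away, then removes itself.
; Each Tick, if the first player controller is valid, it moves to the impact point of a Visibility trace under the cursor.
; It lowers the sprite's alpha at a constant rate scaled by delta time and destroys the actor once nearly transparent.
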(event EventTick
  (params (DeltaSeconds :type Float%20%28single-precision%29))
  (bind _rendercomponent (Variables|Default|GetRenderComponent))
  (bind _spritecolor (Variables|/Script/Paper2D.PaperSpriteComponent|GetSpriteColor _rendercomponent))
  (if (Utilities|IsValid (Game|GetPlayerController 0))
    (Transformation|SetActorLocation (.ImpactPoint (Collision|BreakHitResult (.HitResult (Game|Player|GetHitResultUnderCursorbyChannel (Game|GetPlayerController 0) "TraceTypeQuery1" true)))) false false)
    (Sprite|SetSpriteColor (Variables|Default|GetRenderComponent) (Utilities|Struct|MakeLinearColor (.r _spritecolor) (.g _spritecolor) (.b _spritecolor) (- (.a _spritecolor) (* (Utilities|Time|GetWorldDeltaSeconds) 1.0))))
    (if (not (>= (.a (Variables|/Script/Paper2D.PaperSpriteComponent|GetSpriteColor (Variables|Default|GetRenderComponent))) 0.1))
      (Actor|DestroyActor))))

(event EventBeginPlay)

(event EventActorBeginOverlap
  (params (OtherActor :type Actor%20Object%20Reference)))

(fn ConstructionScript)