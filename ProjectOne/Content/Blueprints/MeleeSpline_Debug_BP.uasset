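; MeleeSpline_Debug_BP is a short-lived actor, named as a melee spline debug aid, that removes itself shortly after spawning.
; BeginPlay sets a fixed three-second lifetime and resets an elapsed-time counter.
; Tick adds world delta seconds to the counter and destroys the actor once the lifetime is reached.
; The construction script is empty, and the graphs contain no spline or drawing logic.
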(event EventBeginPlay
  (Variables|Default|SetDespawnTime 3.0)
  (Variables|Default|SetTimeElapsed 0.0))

(event Collision|EventActorBeginOverlap
  (params (OtherActor :type Actor%20Object%20Reference)))

(event EventTick
  (params (DeltaSeconds :type Float%20%28single-precision%29))
  (if (>= (Variables|Default|GetTimeElapsed) (Variables|Default|GetDespawnTime))
    (Actor|DestroyActor)
    (else
      (Variables|Default|SetTimeElapsed (+ (Variables|Default|GetTimeElapsed) (Utilities|Time|GetWorldDeltaSeconds))))))

(fn ConstructionScript)