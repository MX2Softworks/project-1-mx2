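; Enemy attack event handler that spawns the first attack pattern when its owning GameCharacter triggers an attack.
; On BeginPlay it binds to the owner's OnAttack1 event, which spawns the AttackPattern1 class at a fixed transform rather than the owner's location.
; If the spawn is an OrbPattern_BP and the owner a Sluagh, it copies the pattern's duration into the Sluagh's first attack time and prints a debug message.
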(event Custom|CustomEvent_0
  (bind _returnvalue (Game|SpawnActorfromClass (Variables|Default|GetAttackPattern_1) (Math|Transform|MakeTransform "0, 0,20.000000" "0, 0, 0" "1,1,1") "Undefined" 0 0))
  (bind _asorb_pattern_bp (Utilities|Casting|CastToOrbPattern_BP _returnvalue))
  (bind _assluagh (Utilities|Casting|CastToSluagh (Components|GetOwner)))
  (Class|Sluagh|SetAttackTime1 _assluagh (Variables|/Game/Blueprints/OrbPatterns/OrbPattern_BP.OrbPattern_BP_C|GetPatternTime _asorb_pattern_bp))
  (Development|PrintText "Attack Time Set"))

(event EventBeginPlay
  (bind _asgame_character (Utilities|Casting|CastToGameCharacter (Components|GetOwner)))
  (EventDispatchers|BindEventtoOnAttack1 _asgame_character (delegate Custom|CustomEvent_0)))