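; SoulOrb_BP is a soul orb actor that travels a curve-driven horizontal path and is removed by a SoulTerminator_BP.
; On BeginPlay it caches its spawn location, then Timeline_0 sets its position from the Movement vector curve as a scaled X/Y offset from that point, without sweeping.
; On any actor overlap it waits briefly, then destroys itself only if the other actor casts to SoulTerminator_BP.
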(event EventBeginPlay
  (Variables|Default|SetSpawnLocation (Transformation|GetActorLocation))
  (bind _movement (Timeline|Timeline_0 PlayFromStart)
    (:Update
      (Transformation|SetActorLocation (+ (* (Math|Vector|MakeVector (* (.x _movement) 16.0) (* (.y _movement) 4.0) 0.0) 4e+01) (Variables|Default|GetSpawnLocation)) false false))))

(event Collision|EventActorBeginOverlap
  (params (OtherActor :type Actor%20Object%20Reference))
  (Utilities|FlowControl|Delay 0.3)
  (Utilities|Casting|CastToSoulTerminator_BP OtherActor)
  (Actor|DestroyActor))

(fn ConstructionScript)