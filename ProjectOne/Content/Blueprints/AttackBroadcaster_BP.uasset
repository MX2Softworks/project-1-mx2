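; AttackBroadcaster is a component that turns its owning GameCharacter's first attack event into a spawned attack, in what appears to be a turn-based game.
; On BeginPlay it binds to OnAttack1, then branches on the owner's type when that fires.
; Enemies spawn AttackPattern1; Sluagh owners then derive their attack time from the pattern's duration plus padding and hide the turn order widgets.
; A MainCharacter instead spawns a MeleeDrawer configured for a single swing.
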(event Custom|CustomEvent_0
  (Utilities|Casting|CastToEnemy (stale EventBeginPlay _asgame_character)
    (:then
      (bind _returnvalue (Game|SpawnActorfromClass (Variables|Default|GetAttackPattern_1) (Math|Transform|MakeTransform "0, 0,20.000000" "0, 0, 0" "1,1,1") "Undefined" 0 0))
      (bind _assluagh (Utilities|Casting|CastToSluagh (Components|GetOwner)))
      (Class|Sluagh|SetAttackTime1 _assluagh (+ (Variables|/Game/Blueprints/OrbPatterns/OrbPattern_BP.OrbPattern_BP_C|GetPatternTime _returnvalue) 1.5))
      (Development|PrintText "Attack Time Set")
      (bind _foundwidgets (Widget|GetAllWidgetsOfClass "/Game/Blueprints/Widgets/TurnOrderWidget_BP.TurnOrderWidget_BP_C" true))
      (Widget|SetVisibility _foundwidgets "Hidden"))
    (:CastFailed
      (Utilities|Casting|CastToMainCharacter (stale EventBeginPlay _asgame_character))
      (Game|SpawnActorfromClass "/Game/Blueprints/MeleeDrawer_BP.MeleeDrawer_BP_C" (Math|Transform|MakeTransform "0, 0,20.000000" "0, 0, 0" "1,1,1") "Undefined" 0 0.0 35.0 1))))

(event EventBeginPlay
  (bind _asgame_character (Utilities|Casting|CastToGameCharacter (Components|GetOwner)))
  (EventDispatchers|BindEventtoOnAttack1 _asgame_character (delegate Custom|CustomEvent_0)))