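; Orb pattern spawner that creates SoulOrb_BP actors along a timeline-driven pattern, positioned relative to the battle camera's view.
; On BeginPlay it derives a vertical half-angle from the camera FOV and viewport aspect ratio, then plays SpawnTimeline.
; Each timeline update traces down from the view target, shifts the hit along negative X by distance times that angle's tangent, adds the SpawnPositions value, prints the location and spawns an orb.
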(event EventBeginPlay
  (bind _vertical_fov (CallFunction|GetVerticalFOV))
  (Variables|Default|SetVerticalFOV _vertical_fov)
  (bind _spawnpositions (Timeline|Spawn%20Timeline Play)
    (:Update
      (CallFunction|SpawnOrb _spawnpositions))))

(fn ConstructionScript)

(fn GetVerticalFOV
  (bind _returnvalue (Game|GetPlayerController 0))
  (bind (_sizex _sizey) (HUD|GetViewportSize _returnvalue))
  ;[1 1 1] Calculates Vertical Field of View using the formula V = 2arctan(tan(H/2) * h/w)
  (return (Class|KismetMathLibrary|DegAtan (* (Math|Trig|Tan(Degrees) (/ (Camera|GetFOVAngle (Variables|/Script/Engine.PlayerController|GetPlayerCameraManager _returnvalue)) 2.0)) (/ (Math|Conversions|ToFloat(Integer) _sizey) (Math|Conversions|ToFloat(Integer) _sizex))))))

(fn SpawnOrb
  (params (B :type Vector))
  ;[1 1 1] Casts a trace line from the middle of the screen down to the floor.
  (bind _asbattle_player_controller_bp (Utilities|Casting|CastToBattlePlayerController_BP (Game|GetPlayerController 0))
    (:then
      (bind _outhit (Collision|LineTraceByChannel (Transformation|GetActorLocation (Pawn|GetViewTarget _asbattle_player_controller_bp)) (Math|Vector|MakeVector (.X (Math|Vector|BreakVector (Transformation|GetActorLocation (Pawn|GetViewTarget _asbattle_player_controller_bp)))) (.Y (Math|Vector|BreakVector (Transformation|GetActorLocation (Pawn|GetViewTarget _asbattle_player_controller_bp)))) (- (.Z (Math|Vector|BreakVector (Transformation|GetActorLocation (Pawn|GetViewTarget _asbattle_player_controller_bp)))) 1e+04)) "TraceTypeQuery1" false 0 "None"))
      (Development|PrintText (Utilities|Text|ToText(Name) (Utilities|String|StringToName (Utilities|String|ToString(Vector) (+ (- (.Location (Collision|BreakHitResult _outhit)) (Math|Vector|MakeVector (* (Math|Vector|VectorLength (- (.TraceStart (Collision|BreakHitResult _outhit)) (.Location (Collision|BreakHitResult _outhit)))) (Math|Trig|Tan(Degrees) (Variables|Default|GetVerticalFOV))) 0.0 0.0)) B)))) true true "(R=0.000000,G=0.660000,B=1.000000,A=1.000000)" 1e+01)
      (Game|SpawnActorfromClass "/Game/Blueprints/SoulOrb_BP.SoulOrb_BP_C" (Math|Transform|MakeTransform (+ (- (.Location (Collision|BreakHitResult _outhit)) (Math|Vector|MakeVector (* (Math|Vector|VectorLength (- (.TraceStart (Collision|BreakHitResult _outhit)) (.Location (Collision|BreakHitResult _outhit)))) (Math|Trig|Tan(Degrees) (Variables|Default|GetVerticalFOV))) 0.0 0.0)) B) "0.000000,0.000000,90.000000" "0.250000,1.000000,0.250000") "AlwaysSpawn" 0 0)
      (return))
    (:CastFailed
      (return))))