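; SoulOrb_BP is an animated soul orb that travels from its spawn point and disappears when it reaches a SoulTerminator_BP.
; A timeline started on BeginPlay drives its X/Y position as a scaled offset from the spawn location, while a looping Paper flipbook animates it.
; Overlapping a terminator destroys it after a short delay.
; Clicking it only prints the mouse's deprojected world position via BattlePlayerController_BP.
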(event EventBeginPlay
  (Variables|Default|SetSpawnLocation (Transformation|GetActorLocation))
  (Components|Timeline|SetLooping (Variables|Default|GetPaperFlipbook) true)
  (bind _movement (Timeline|Timeline_1 PlayFromStart)
    (:Update
      (Transformation|SetActorLocation (+ (* (Math|Vector|MakeVector (* (.x _movement) 16.0) (* (.y _movement) 4.0) 0.0) 4e+01) (Variables|Default|GetSpawnLocation)) false false))))

(event MouseInput|EventActorOnClicked
  (bind _asbattle_player_controller_bp (Utilities|Casting|CastToBattlePlayerController_BP (Game|GetPlayerController 0)))
  (Development|PrintText (Utilities|Text|ToText(String) (Utilities|String|ToString(Vector) (.WorldLocation (Game|Player|ConvertMouseLocationToWorldSpace _asbattle_player_controller_bp))))))

(event Collision|EventActorBeginOverlap
  (params (OtherActor :type Actor%20Object%20Reference))
  (Utilities|Casting|CastToSoulTerminator_BP OtherActor)
  (Utilities|FlowControl|Delay 0.3)
  (Actor|DestroyActor))

(event EventTick
  (params (DeltaSeconds :type Float%20%28single-precision%29))
  (Audio|Components|Audio|Play (Variables|Default|GetPaperFlipbook)))

(fn ConstructionScript)