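; Mouse-driven reticle actor that highlights soul orbs beneath it and destroys them on left click.
; Each tick it moves to the cursor's hit location at a fixed height, using the battle player controller.
; Overlaps maintain an array of orbs and swap their flipbooks, reapplying playback position; clicking destroys and clears that array.
; BeginPlay also enables input, sets rotation and traces for a floor distance that is never read here.
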(event Collision|EventActorEndOverlap
  (params (OtherActor :type Actor%20Object%20Reference))
  (bind _assoul_orb_bp (Utilities|Casting|CastToSoulOrb_BP OtherActor))
  (Utilities|Array|RemoveItem (Variables|Default|GetOverlapActorArray) _assoul_orb_bp)
  (Sprite|SetFlipbook (Variables|/Game/Blueprints/SoulOrb_BP.SoulOrb_BP_C|GetPaperFlipbook _assoul_orb_bp) "/Game/Assets/Flipbooks/SoulOrb_Default/Soul_Orb.Soul_Orb")
  (Components|Timeline|SetNewTime (Variables|/Game/Blueprints/SoulOrb_BP.SoulOrb_BP_C|GetPaperFlipbook _assoul_orb_bp) (Components|Timeline|GetPlaybackPosition (Variables|/Game/Blueprints/SoulOrb_BP.SoulOrb_BP_C|GetPaperFlipbook _assoul_orb_bp))))

(event EventBeginPlay
  (bind _asbattle_player_controller_bp (Utilities|Casting|CastToBattlePlayerController_BP (Game|GetPlayerController 0)))
  (Input|EnableInput _asbattle_player_controller_bp)
  (bind _asbattle_player_controller_bp_2 (Utilities|Casting|CastToBattlePlayerController_BP (Game|GetPlayerController 0)))
  (Variables|Default|SetMyPlayerCharacterReference _asbattle_player_controller_bp_2)
  (Transformation|SetActorRotation "0.000000,90.000000,90.000000")
  (bind _outhit (Collision|LineTraceByChannel (.WorldLocation (Game|Player|ConvertMouseLocationToWorldSpace _asbattle_player_controller_bp_2)) (- (.WorldLocation (Game|Player|ConvertMouseLocationToWorldSpace _asbattle_player_controller_bp_2)) "0, 0,-5000.000000") "TraceTypeQuery1" false 0 "None"))
  (if (Utilities|Enum|Equal(Enum) (Utilities|GetObjectName (.HitActor (Collision|BreakHitResult _outhit))) "floor")
    (Variables|Default|SetFloorLength (.z (- (.TraceStart (Collision|BreakHitResult _outhit)) (Math|Vector|MakeVector 0.0 0.0 (+ (.z (Transformation|GetActorLocation (.HitActor (Collision|BreakHitResult _outhit)))) 1e+01)))))))

(event EventTick
  (params (DeltaSeconds :type Float%20%28single-precision%29))
  (bind _myplayercharacterreference (Variables|Default|GetMyPlayerCharacterReference))
  (bind _hitresult (Game|Player|GetHitResultUnderCursorbyChannel _myplayercharacterreference "TraceTypeQuery1" true))
  (bind _location (Collision|BreakHitResult _hitresult))
  (if (Utilities|IsValid (Variables|Default|GetMyPlayerCharacterReference))
    (Transformation|SetActorLocation (Math|Vector|MakeVector (.x _location) (.y _location) 1e+02) false false)))

(event Collision|EventActorBeginOverlap
  (params (OtherActor :type Actor%20Object%20Reference))
  (bind _assoul_orb_bp (Utilities|Casting|CastToSoulOrb_BP OtherActor))
  (Utilities|Array|AddUnique (Variables|Default|GetOverlapActorArray) _assoul_orb_bp)
  (Sprite|SetFlipbook (Variables|/Game/Blueprints/SoulOrb_BP.SoulOrb_BP_C|GetPaperFlipbook _assoul_orb_bp) "/Game/Assets/Flipbooks/SoulOrb_Default_Highlighted/Soul_Orb_Highlighted.Soul_Orb_Highlighted")
  (Components|Timeline|SetNewTime (Variables|/Game/Blueprints/SoulOrb_BP.SoulOrb_BP_C|GetPaperFlipbook _assoul_orb_bp) (Components|Timeline|GetPlaybackPosition (Variables|/Game/Blueprints/SoulOrb_BP.SoulOrb_BP_C|GetPaperFlipbook _assoul_orb_bp))))

(event Input|MouseEvents|LeftMouseButton
  (params (Key :type Key%20Structure :default "AnyKey"))
  (:Pressed
    (for _array_element (Variables|Default|GetOverlapActorArray)
      (if (Utilities|IsValid _array_element)
        (Actor|DestroyActor _array_element)))
    (Utilities|Array|Clear (Variables|Default|GetOverlapActorArray))))

(fn ConstructionScript)